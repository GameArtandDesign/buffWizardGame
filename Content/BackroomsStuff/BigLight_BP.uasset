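; BigLight_BP is a Backrooms light that flickers endlessly by driving the intensity of its W1 light.
; Tick passes a DoOnce into a chain of fresh random rolls that picks one of six timelines unevenly, and each timeline resets the gate when finished.
; Each update scales the curve by a random offset factor and widens its Min/Max range with no reset, so flicker variance grows over time.
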(event `self.ReceiveTick`
  (params (DeltaSeconds :type "Float (single-precision)"))
  (bind _returnvalue (`KismetMathLibrary.RandomIntegerInRange` 0 5))
  (bind _returnvalue_2 (+ (`KismetMathLibrary.RandomFloatInRange` (`self.min`) (`self.max`)) 2.0))
  (`/Engine/EditorBlueprintResources/StandardMacros.DoOnce` false :!label _label
    (:`Completed`
      (if (== _returnvalue 0)
        (bind (_direction _newtrack_0) (`Timeline|Timeline_4` :!via `PlayFromStart`)
          (:`Update`
            (`LightComponent.SetIntensity` (`self.w1`) (* _newtrack_0 _returnvalue_2)))
          (:`Finished`
            (goto _label :!via `Reset`)))
        (elif (== _returnvalue 1)
          (bind (_direction_2 _newtrack_0_2) (`Timeline|Timeline_3` :!via `PlayFromStart`)
            (:`Update`
              (`LightComponent.SetIntensity` (`self.w1`) (* _newtrack_0_2 _returnvalue_2)))
            (:`Finished`
              (goto _label :!via `Reset`)))
          (elif (== _returnvalue 2)
            (bind (_direction_3 _newtrack_0_3) (`Timeline|Timeline_2` :!via `PlayFromStart`)
              (:`Update`
                (`LightComponent.SetIntensity` (`self.w1`) (* _newtrack_0_3 _returnvalue_2)))
              (:`Finished`
                (goto _label :!via `Reset`)))
            (elif (== _returnvalue 3)
              (bind (_direction_4 _newtrack_0_4) (`Timeline|Timeline_1` :!via `PlayFromStart`)
                (:`Update`
                  (`LightComponent.SetIntensity` (`self.w1`) (* _newtrack_0_4 _returnvalue_2)))
                (:`Finished`
                  (goto _label :!via `Reset`)))
              (elif (== _returnvalue 4)
                (bind (_direction_5 _newtrack_0_5) (`Timeline|Timeline_0` :!via `PlayFromStart`)
                  (:`Update`
                    (`LightComponent.SetIntensity` (`self.w1`) (* _newtrack_0_5 _returnvalue_2)))
                  (:`Finished`
                    (goto _label :!via `Reset`)))
                (else
                  (bind (_direction_6 _newtrack_0_6) (`Timeline|Timeline` :!via `PlayFromStart`)
                    (:`Update`
                      (`LightComponent.SetIntensity` (`self.w1`) (* _newtrack_0_6 _returnvalue_2)))
                    (:`Finished`
                      (goto _label :!via `Reset`)))))))))
      (set `self.min` (- (`self.min`) 0.0005))
      (set `self.max` (+ (`self.max`) 0.0005)))))

(fn `UserConstructionScript`)